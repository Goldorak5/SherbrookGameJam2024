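; BP_BiberonStands is a baby bottle warming stand that shows a progress bar widget and an interaction nameplate.
; On BeginPlay it links the progress bar to itself and its serial number, then starts heating automatically.
; After a delay, a Timeline drives HeatTime from zero to its maximum.
; A sphere overlap with BP_Adulte toggles the "(Q) Chauffé Biberon" prompt and CanInteract, though no input is handled here.
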(event `self.ReceiveBeginPlay`
  (bind _aswb_biberon_progresse_bar (cast `/Game/Blueprint/Biberon/Biberon_V0/WB_BiberonProgresseBar` (`WidgetComponent.GetUserWidgetObject` (`self.ProgresseBar`))))
  (set `/Game/Blueprint/Biberon/Biberon_V0/WB_BiberonProgresseBar.BiberonStands` self _aswb_biberon_progresse_bar)
  (bind _aswb_biberon_name_plate (cast `/Game/Blueprint/Biberon/Biberon_V0/WB_BiberonNamePlate` (`WidgetComponent.GetUserWidgetObject` (`self.NamePlate`))))
  (`TextBlock.SetText` (`/Game/Blueprint/Biberon/Biberon_V0/WB_BiberonNamePlate.Nameplate` _aswb_biberon_name_plate) "(Q) Chauffé Biberon")
  (`SceneComponent.SetVisibility` (`self.NamePlate`) false false)
  (bind _aswb_biberon_progresse_bar_2 (cast `/Game/Blueprint/Biberon/Biberon_V0/WB_BiberonProgresseBar` (`WidgetComponent.GetWidget` (`self.ProgresseBar`))))
  (set `/Game/Blueprint/Biberon/Biberon_V0/WB_BiberonProgresseBar.SerialNumber` (`self.SerialNumber`) _aswb_biberon_progresse_bar_2)
  (`self.StartHeating`))

(event `self.Sphere.OnComponentBeginOverlap`
  (params (OverlappedComponent :type "PrimitiveComponent Object Reference") (OtherActor :type "Actor Object Reference") (OtherComp :type "PrimitiveComponent Object Reference") (OtherBodyIndex :type Integer) (bFromSweep :type Boolean) (SweepResult :type "HitResult Structure (by ref)"))
  (cast `/Game/ThirdPerson/Blueprints/BP_Adulte` OtherActor
    (:`then`
      (`KismetSystemLibrary.PrintString` "Hello")
      (`SceneComponent.SetVisibility` (`self.NamePlate`) true false)
      (set `self.CanInteract` true))
    (:`CastFailed`
      (`KismetSystemLibrary.PrintString` "fail"))))

(event `self.Sphere.OnComponentEndOverlap`
  (params (OverlappedComponent :type "PrimitiveComponent Object Reference") (OtherActor :type "Actor Object Reference") (OtherComp :type "PrimitiveComponent Object Reference") (OtherBodyIndex :type Integer))
  (cast `/Game/ThirdPerson/Blueprints/BP_Adulte` OtherActor)
  (`SceneComponent.SetVisibility` (`self.NamePlate`) false false)
  (set `self.CanInteract` false))

(event `StartHeating`
  (`KismetSystemLibrary.Delay` (`self.wait`))
  (bind (_direction _chauffer) (`Timeline|Timeline` :!via `PlayFromStart`)
    (:`Update`
      (set `self.HeatTime` (`KismetMathLibrary.Lerp` 0.0 (`self.MaxHeatTime`) _chauffer)))))

(fn `UserConstructionScript`)