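; Baby AI that randomly roams or seeks out dangerous objects and hurts itself unless carried in time.
; Tick drives an enum state machine with bool guards, launching AIMoveTo roaming and danger events.
; The reached object's type selects looping damage or a delayed one-shot kill, both timer-based and cleared on pickup.
; Tick destroys the baby near zero life and notifies BP_EndGameManager; a progress bar widget references the baby.
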(event `self.ReceiveBeginPlay`
  ;[1 1 1] Initialisation
  (bind _aswb_baby_progresse_bar (cast `/Game/Blueprint/UI/WB_BabyProgresseBar` (`WidgetComponent.GetWidget` (`self.BabyProgresseBar`))))
  (set `/Game/Blueprint/UI/WB_BabyProgresseBar.BabyOwner` self _aswb_baby_progresse_bar)
  (set `self.life` (`self.maxLife`))
  (set `self.Player` (`GameplayStatics.GetPlayerPawn` 0))
  (set `self.StateMachine` "NewEnumerator0")
  (bind _outactors (`GameplayStatics.GetAllActorsOfClass` "/Game/Blueprint/BP_EndGameManager.BP_EndGameManager_C"))
  (for _array_element _outactors
    (set `self.As BP End Game Manager` _array_element)))

(event `self.ReceiveTick`
  (params (DeltaSeconds :type "Float (single-precision)"))
  ;[1 1 1] Behavior
  (if (`KismetMathLibrary.NearlyEqual_FloatFloat` (`self.life`) 0.0 0.5)
    (`self.K2_DestroyActor`)
    (`/Game/Blueprint/BP_EndGameManager.BabyDeath` (`self.As BP End Game Manager`))
    (else
      (switch `/Game/Blueprint/Enum_BabyStates` (`self.StateMachine`)
        (:`NewEnumerator0`
          ;;[1 1 1] Is Roaming
          (if (not (`self.isRoaming`))
            (set `self.isRoaming` true)
            (`self.Random Roam`)))
        (:`NewEnumerator1`
          ;;[1 1 1] Is in Danger
          (if (`self.isGettingCarried`)
            (set `self.StateMachine` "NewEnumerator2")
            (set `self.isInDanger` false)
            (elif (not (`self.isInDanger`))
              (set `self.isInDanger` true)
              (`self.DangerEvent`))))
        (:`NewEnumerator2`
          ;;[1 1 1] Is safe
          (if (not (`self.isSafe`))
            (set `self.isSafe` true)
            (if (== (`self.CurrentDanger`) 0)
              (`self.Stop Hurting Himself 1`)
              (else
                (`self.Stop Hurting Himself Type 2`)))
            (set `self.StateMachine` "NewEnumerator0")
            (set `self.isSafe` false)))
        (:`NewEnumerator3`
          ;;[1 1 1] Is Hurting
          (if (`self.isHurtingHimself`)
            _
            (elif (== (`self.CurrentDanger`) 0)
              (`self.Hurting Himself Type 1Event`)
              (else
                (`self.Hurting Himself Type 2`)))))))))

(event `Random Roam`
  ;[1 1 1] Roaming State
  (if (>= (`KismetMathLibrary.RandomInteger` 100) 50)
    (`|AIMoveTo` self (`NavigationSystemV1.K2_GetRandomReachablePointInRadius` (`self.K2_GetActorLocation`) 2500.0 null null) null
      (:`OnSuccess`
        _)
      (:`OnFail`
        _))
    (`self.Random Roam`)
    (else
      (set `self.StateMachine` "NewEnumerator1"))))

(event `DangerEvent`
  ;[1 1 1] DangerState
  (bind _output_get (set `self.DangerChoisi` (`KismetArrayLibrary.Array_Random` (`self.Danger`))))
  (`|AIMoveTo` self (0.0 0.0 0.0) _output_get
    (:`then`
      (bind _asbp_dangerous_object_instant (cast `/Game/Blueprint/priseElectrique/BP_DangerousObjectInstant` _output_get)
        (:`then`
          (set `self.CurrentDanger` (`/Game/Blueprint/priseElectrique/BP_DangerousObjectInstant.Object type` _asbp_dangerous_object_instant))
          (set `self.DangerChoisi` null))
        (:`CastFailed`
          (bind _asbp_dangerous_object_instant_2 (cast `/Game/Blueprint/Couteau/BP_DangerousObjectInstant2` _output_get)
            (:`then`
              (set `self.CurrentDanger` (`/Game/Blueprint/Couteau/BP_DangerousObjectInstant2.Object type` _asbp_dangerous_object_instant_2))
              (set `self.DangerChoisi` null))
            (:`CastFailed`
              (bind _asbp_bleach (cast `/Game/Blueprint/Bleach/BP_bleach` _output_get))
              (set `self.CurrentDanger` (`/Game/Blueprint/Bleach/BP_bleach.Object type` _asbp_bleach))
              (set `self.DangerChoisi` null))))))
    (:`OnSuccess`
      (set `self.StateMachine` "NewEnumerator3")
      (set `self.isInDanger` false))))

(event `heal`
  (set `self.life` (`self.maxLife`)))

(event `IsCarried`
  (params (isGettingCarried :type Boolean))
  ;[1 1 1] Is carried
  (set `self.isGettingCarried` isGettingCarried)
  (`self.Stop Hurting Himself 1`)
  (`self.Stop Hurting Himself Type 2`))

(event `Hurting Himself Type 1Event`
  ;[1 1 1] Hurting Himself type 1 State
  (set `self.isHurtingHimself` true)
  (bind _returnvalue (`KismetSystemLibrary.K2_SetTimerDelegate` (delegate `TakeDamage`) 0.1 true))
  (if (`self.isGettingCarried`)
    (set `self.Electrocution` false)
    (set `self.StateMachine` "NewEnumerator2")
    (set `self.isHurtingHimself` false)))

(event `TakeDamage`
  ;[1 1 1] Hurting Himself type 1 State
  (set `self.Electrocution` true)
  (set `self.isHurtingHimself` true)
  (set `self.life` (- (`self.life`) 1.0)))

(event `Stop Hurting Himself 1`
  ;[1 1 1] Hurting Himself type 1 State
  (set `self.isHurtingHimself` false)
  (`KismetSystemLibrary.K2_ClearAndInvalidateTimerHandle` (stale `Hurting Himself Type 1Event` _returnvalue)))

(event `Hurting Himself Type 2`
  ;[1 1 1] Hurting Himself type 2 State
  (set `self.Mort_Instant` true)
  (set `self.isHurtingHimself` true)
  (bind _returnvalue (`KismetSystemLibrary.K2_SetTimerDelegate` (delegate `oneShot`) 5.0 true))
  (if (`self.isGettingCarried`)
    (set `self.Mort_Instant` false)
    (set `self.StateMachine` "NewEnumerator2")
    (set `self.isHurtingHimself` false)))

(event `Stop Hurting Himself Type 2`
  ;[1 1 1] Hurting Himself type 2 State
  (set `self.isHurtingHimself` false)
  (`KismetSystemLibrary.K2_ClearAndInvalidateTimerHandle` (stale `Hurting Himself Type 2` _returnvalue)))

(event `oneShot`
  (bind _returnvalue_location (`KismetMathLibrary.BreakTransform` (`self.GetTransform`)))
  ;[1 1 1] Hurting Himself type 2 State
  (set `self.isHurtingHimself` true)
  (`GameplayStatics.PlaySoundAtLocation` "/Game/Sounds/SFX_Knife.SFX_Knife" _returnvalue_location (struct) 1.0 1.0 0.0 null null null null)
  (set `self.life` 0.0))

(fn `UserConstructionScript`)