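; BP_Baby is an AI-driven baby that wanders until it seeks out a dangerous object and hurts itself.
; An enum state machine, checked every Tick with once-only flags, starts behaviors and destroys the actor near zero Life.
; Roaming chains random AI moves, with a 1% chance per move of targeting a random Danger actor.
; The object's type selects one of two hurt timelines that affect Life or switch to Safe, which stops only the first.
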(event `self.ReceiveBeginPlay`
  (set `self.life` 100.0)
  (set `self.StateMachine` "NewEnumerator0")
  (if (`KismetMathLibrary.NearlyEqual_FloatFloat` (`self.life`) 0.0 0.5) :!label _label
    (`self.K2_DestroyActor`)
    (else
      (switch `/Game/Blueprint/Enum_BabyStates` (`self.StateMachine`)
        (:`NewEnumerator0`
          (if (not (`self.isRoaming`))
            (`self.Random Roam`)
            (set `self.isRoaming` true)))
        (:`NewEnumerator1`
          (if (not (`self.isInDanger`))
            (`self.DangerEvent`)
            (set `self.isInDanger` true)))
        (:`NewEnumerator2`
          (if (not (`self.isSafe`))
            (`self.Stop Hurting Himself 1`)
            (`KismetSystemLibrary.PrintString` "Safe")
            (set `self.isSafe` true)))
        (:`NewEnumerator3`
          (if (`self.isHurtingHimself`)
            _
            (elif (== (`self.CurrentDanger`) 0)
              (`self.Hurting Himself Type 1Event`)
              (set `self.isHurtingHimself` true)
              (else
                (`self.Hurting Himself Type 2`)
                (set `self.isHurtingHimself` true)))))))))

(event `self.ReceiveTick`
  (params (DeltaSeconds :type "Float (single-precision)"))
  (goto _label))

(event `Random Roam`
  ;[1 1 1] Roaming State
  (if (>= (`KismetMathLibrary.RandomInteger` 100) 1)
    (`|AIMoveTo` self (`NavigationSystemV1.K2_GetRandomReachablePointInRadius` (`self.K2_GetActorLocation`) 2500.0 null null) null
      (:`OnSuccess`
        _)
      (:`OnFail`
        _))
    (`self.Random Roam`)
    (else
      (`self.DangerEvent`)
      (set `self.isHurtingHimself` false))))

(event `DangerEvent`
  ;[1 1 1] DangerState
  (bind _output_get (set `self.current Actor` (`KismetArrayLibrary.Array_Random` (`self.Danger`))))
  (`|AIMoveTo` self (0.0 0.0 0.0) _output_get
    (:`then`
      (bind _asbp_dangerous_object_instant (cast `/Game/Blueprint/BP_DangerousObjectInstant` _output_get))
      (bind _output_get_2 (set `self.CurrentDanger` (`/Game/Blueprint/BP_DangerousObjectInstant.Object type` _asbp_dangerous_object_instant)))
      (`KismetSystemLibrary.PrintText` (`KismetTextLibrary.Conv_IntToText` _output_get_2)))
    (:`OnSuccess`
      (set `self.StateMachine` "NewEnumerator3"))))

(event `Hurting Himself Type 1Event`
  ;[1 1 1] Hurting Himself type 1 State
  (bind (_direction _lifedrain) (`Timeline|HurtingHimself` :!via `PlayFromStart` :!label _label_2)
    (:`Update`
      (bind _output_get (set `self.life` (`KismetMathLibrary.Lerp` 0.0 100.0 _lifedrain)))
      (if (<= _output_get 50.0)
        (set `self.StateMachine` "NewEnumerator2")))))

(event `Stop Hurting Himself 1`
  ;[1 1 1] Hurting Himself type 1 State
  (goto _label_2 :!via `Stop`))

(event `Hurting Himself Type 2`
  ;[1 1 1] Hurting Himself type 2 State
  (`KismetSystemLibrary.PrintString` "Type 2 !!")
  (bind (_direction _lifedrain) (`Timeline|Timeline` :!via `PlayFromStart` :!label _label_3)
    (:`Update`
      (if true
        (set `self.StateMachine` "NewEnumerator2")))
    (:`Finished`
      (set `self.life` 0.0))))

(event `Stop Hurting Himself Type 2`
  ;[1 1 1] Hurting Himself type 2 State
  (goto _label_3 :!via `Stop`))

(fn `UserConstructionScript`)