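; BP_Camera toggles the view between an external camera and the player's BP_Adulte2 character.
; Its SwitchCamera event flips IsOn and sets the player controller's view target to ExternalCamera when turning off, or to the character when turning on.
; It then copies IsOn into the character's IsExternalCamera, so that flag is true while the character, not the external camera, is the view target.
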(event `SwitchCamera`
  (bind _returnvalue (`GameplayStatics.GetPlayerController` 0))
  (bind _asbp_adulte (cast `/Game/ThirdPerson/Blueprints/BP_Adulte2` (`GameplayStatics.GetPlayerCharacter` 0)))
  (if (`self.isOn`)
    (set `self.isOn` false)
    (`PlayerController.SetViewTargetWithBlend` _returnvalue (`self.ExternalCamera`) 0.0 "VTBlend_Linear" 0.0 false)
    (else
      (set `self.isOn` true)
      (`PlayerController.SetViewTargetWithBlend` _returnvalue _asbp_adulte 0.0 "VTBlend_Linear" 0.0 false)))
  (bind _asbp_adulte_2 (cast `/Game/ThirdPerson/Blueprints/BP_Adulte2` (`GameplayStatics.GetPlayerCharacter` 0)))
  (set `/Game/ThirdPerson/Blueprints/BP_Adulte2.isExternalCamera` (`self.isOn`) _asbp_adulte_2))

(fn `UserConstructionScript`)