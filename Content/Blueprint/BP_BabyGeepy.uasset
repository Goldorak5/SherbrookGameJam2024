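; BP_BabyGeepy is an AI baby creature that heads into dangers and loses life until destroyed.
; An enum state machine, run on BeginPlay and Tick, covers roaming, danger detected, safe (print only) and self-hurting.
; RandomRoam's random check never passes, so it always moves to a random Danger actor, then switches to self-hurting.
; There a one-shot timeline sets Life, and the actor is destroyed near zero.
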(event `Random Roam`
  (if (>= (`KismetMathLibrary.RandomInteger` 100) 100)
    (`|AIMoveTo` self (`NavigationSystemV1.K2_GetRandomReachablePointInRadius` (`self.K2_GetActorLocation`) 2500.0 null null) null
      (:`OnSuccess`
        _)
      (:`OnFail`
        _))
    (`self.Random Roam`)
    (else
      (`|AIMoveTo` self (0.0 0.0 0.0) (`KismetArrayLibrary.Array_Random` (`self.Danger`))
        (:`OnSuccess`
          (set `self.isHurtingHimself` false)
          (set `self.StateMachine` "NewEnumerator3"))))))

(event `self.ReceiveBeginPlay`
  (set `self.life` 100.0)
  (set `self.StateMachine` "NewEnumerator0")
  (if (`KismetMathLibrary.NearlyEqual_FloatFloat` (`self.life`) 0.0 0.5) :!label _label
    (`self.K2_DestroyActor`)
    (else
      (switch `/Game/Blueprint/Enum_BabyStates` (`self.StateMachine`)
        (:`NewEnumerator0`
          (if (not (`self.isRoaming`))
            (`self.Random Roam`)
            (set `self.isRoaming` true)))
        (:`NewEnumerator1`
          (if (not (`self.isInDanger`))
            (set `self.isInDanger` true)
            (`|AIMoveTo` self (0.0 0.0 0.0) (`KismetArrayLibrary.Array_Random` (`self.Danger`))
              (:`OnSuccess`
                (set `self.StateMachine` "NewEnumerator3")))))
        (:`NewEnumerator2`
          (`KismetSystemLibrary.PrintString` "Safe"))
        (:`NewEnumerator3`
          (if (not (`self.isHurtingHimself`))
            (`/Engine/EditorBlueprintResources/StandardMacros.DoOnce` false
              (:`Completed`
                (set `self.isHurtingHimself` true)
                (bind (_direction _lifedrain) (`Timeline|HurtingHimself` :!via `PlayFromStart`)
                  (:`Update`
                    (set `self.life` (`KismetMathLibrary.Lerp` 0.0 100.0 _lifedrain))
                    (`KismetSystemLibrary.PrintText` (`KismetTextLibrary.Conv_DoubleToText` (`self.life`) "HalfToEven"))))))))))))

(event `self.ReceiveTick`
  (params (DeltaSeconds :type "Float (single-precision)"))
  (goto _label))

(fn `UserConstructionScript`)