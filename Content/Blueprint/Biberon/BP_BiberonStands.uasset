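; Baby bottle (biberon) warming stand that adult players can approach to heat a bottle.
; BeginPlay passes itself to the progress bar widget and sets a hidden right-click prompt nameplate.
; Sphere overlaps with BP_Adulte toggle the nameplate and CanInteract.
; StartHeating, guarded by IsHeating, runs a Timeline that lerps HeatTime up to MaxHeatTime, then flags BibsReady when finished.
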(event `self.ReceiveBeginPlay`
  (bind _aswb_biberon_progresse_bar (cast `/Game/Blueprint/Biberon/WB_BiberonProgresseBar` (`WidgetComponent.GetUserWidgetObject` (`self.ProgresseBar`))))
  (set `/Game/Blueprint/Biberon/WB_BiberonProgresseBar.BiberonStands` self _aswb_biberon_progresse_bar)
  (bind _aswb_biberon_name_plate (cast `/Game/Blueprint/Biberon/WB_BiberonNamePlate` (`WidgetComponent.GetUserWidgetObject` (`self.NamePlate`))))
  (`TextBlock.SetText` (`/Game/Blueprint/Biberon/WB_BiberonNamePlate.Nameplate` _aswb_biberon_name_plate) "(Click Droit) Chauffé Biberon")
  (`SceneComponent.SetVisibility` (`self.NamePlate`) false false))

(event `self.Sphere.OnComponentBeginOverlap`
  (params (OverlappedComponent :type "PrimitiveComponent Object Reference") (OtherActor :type "Actor Object Reference") (OtherComp :type "PrimitiveComponent Object Reference") (OtherBodyIndex :type Integer) (bFromSweep :type Boolean) (SweepResult :type "HitResult Structure (by ref)"))
  (cast `/Game/ThirdPerson/Blueprints/BP_Adulte` OtherActor)
  (`SceneComponent.SetVisibility` (`self.NamePlate`) true false)
  (set `self.CanInteract` true))

(event `self.Sphere.OnComponentEndOverlap`
  (params (OverlappedComponent :type "PrimitiveComponent Object Reference") (OtherActor :type "Actor Object Reference") (OtherComp :type "PrimitiveComponent Object Reference") (OtherBodyIndex :type Integer))
  (cast `/Game/ThirdPerson/Blueprints/BP_Adulte` OtherActor)
  (`SceneComponent.SetVisibility` (`self.NamePlate`) false false)
  (set `self.CanInteract` false))

(event `StartHeating`
  (if (not (`self.isHeating`))
    (bind (_direction _chauffer) (`Timeline|Timeline` :!via `PlayFromStart`)
      (:`Update`
        (set `self.isHeating` true)
        (set `self.BibsReady` false)
        (set `self.HeatTime` (`KismetMathLibrary.Lerp` 0.0 (`self.MaxHeatTime`) _chauffer)))
      (:`Finished`
        (set `self.BibsReady` true)
        (set `self.isHeating` false)))))

(fn `UserConstructionScript`)